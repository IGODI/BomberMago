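; BP_BomberMago is a playable bomber mage character that spawns a shared or split-screen HUD based on the game instance.
; Attack spawns one of three bombs chosen by Seleçao (magic, tower or AI explosive copy) at a Box whose overlaps block placement; the used-bomb count resets after a delay.
; Tick pins the camera angle and applies walk speed.
; Touching a "Bomba"-tagged actor zeroes health, triggering the end screen and destruction.
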(event OnComponentBeginOverlap(CapsuleComponent)
  (params (OverlappedComponent :type Primitive%20Component%20Object%20Reference) (OtherActor :type Actor%20Object%20Reference) (OtherComp :type Primitive%20Component%20Object%20Reference) (OtherBodyIndex :type Integer) (bFromSweep :type Boolean) (SweepResult :type Hit%20Result%20Structure%20%28by%20ref%29))
  (if (Actor|ActorHasTag OtherActor "Bomba")
    (Variables|Default|SetHealth 0.0)))

(event OnComponentBeginOverlap(Box)
  (params (OverlappedComponent :type Primitive%20Component%20Object%20Reference) (OtherActor :type Actor%20Object%20Reference) (OtherComp :type Primitive%20Component%20Object%20Reference) (OtherBodyIndex :type Integer) (bFromSweep :type Boolean) (SweepResult :type Hit%20Result%20Structure%20%28by%20ref%29))
  ;[1 1 1] Pode Atacar?
  (Variables|Default|SetPodeAtacar false))

(event OnComponentEndOverlap(Box)
  (params (OverlappedComponent :type Primitive%20Component%20Object%20Reference) (OtherActor :type Actor%20Object%20Reference) (OtherComp :type Primitive%20Component%20Object%20Reference) (OtherBodyIndex :type Integer))
  ;[1 1 1] Pode Atacar?
  (Variables|Default|SetPodeAtacar true))

(event EventBeginPlay
  ;[1 1 1] HUD
  (bind _asbp_game_instance (Utilities|Casting|CastToBp_GameInstance (Game|GetGameInstance)))
  (if (Variables|/Game/Marcos/Blueprints/UI/Bp_GameInstance.Bp_GameInstance_C|GetTelaCompartilhada _asbp_game_instance)
    (bind _returnvalue (UserInterface|CreateWidget "/Game/Marcos/Blueprints/UI/HUDS/TelaCompartilhada.TelaCompartilhada_C" (Game|GetPlayerController 0)))
    (UserInterface|Viewport|AddtoViewport _returnvalue 0)
    (else
      (bind _returnvalue_2 (UserInterface|CreateWidget "/Game/Marcos/Blueprints/UI/HUDS/TelaDividida.TelaDividida_C" (Game|GetPlayerController 0)))
      (UserInterface|Viewport|AddtoPlayerScreen _returnvalue_2))))

(event EventTick
  (params (DeltaSeconds :type Float%20%28single-precision%29))
  ;[1 1 1] Vida / Movimento / Camera
  (Transformation|SetRelativeLocation (Variables|Default|GetCamera) "0, 0,607.735046" false false)
  (Transformation|SetWorldRotation (Variables|Default|GetCamera) "-60.000000, 0, 0" false false)
  (Variables|/Script/Engine.CharacterMovementComponent|SetMaxWalkSpeed (Variables|Character|GetCharacterMovement) (Variables|Default|GetVelocidade))
  (if (<= (Variables|Default|GetHealth) 0.0)
    (bind _returnvalue (UserInterface|CreateWidget "/Game/Marcos/Blueprints/UI/HUDS/Fim.Fim_C"))
    (Variables|/Script/Engine.PlayerController|SetbShowMouseCursor (Game|GetPlayerController 0) true)
    (UserInterface|Viewport|AddtoViewport _returnvalue 0)
    (Variables|Default|SetVivo/Morto true)
    (Default|OChamado _returnvalue)
    (Utilities|FlowControl|Delay 0.2)
    (Actor|DestroyActor)))

(event Input|ActionEvents|InputActionAtacar
  (params (Key :type Key%20Structure :default "None"))
  (bind _box (Variables|Default|GetBox))
  (bind _returnvalue (Transformation|GetWorldLocation _box))
  ;[1 1 1] Invocar Bomba
  (:Pressed
    (if (< (Variables|Default|GetBombasGastas) (Variables|Default|GetLimiteBombas))
      (bind _result (Math|Integer|IncrementInt (Variables|Default|GetBombasGastas))
        (:%20%20
          (Variables|Default|SetBombasGastas _result)
          (if (Variables|Default|GetPodeAtacar)
            (switch int (Variables|Default|GetSeleçao)
              (:0
                (Game|SpawnActorfromClass "/Game/Marcos/Blueprints/Bombas/BombaPadrão/BP_BombaMagica.BP_BombaMagica_C" (Math|Transform|MakeTransform _returnvalue "0, 0, 0" "1,1,1") "AdjustIfPossibleButAlwaysSpawn" 0 (Variables|Default|GetForçah) 0))
              (:1
                (Game|SpawnActorfromClass "/Game/Marcos/Blueprints/Bombas/BombaTorre/BP_BombaTorreMagica.BP_BombaTorreMagica_C" (Math|Transform|MakeTransform _returnvalue "0, 0, 0" "1,1,1") "AdjustIfPossibleButAlwaysSpawn" 0 (Variables|Default|GetVelocidadeBala) 0))
              (:2
                (AI|SpawnAIFromClass "/Game/Marcos/Blueprints/Bombas/CopiaExplosiva/BP_BombaCopiaExplosiva.BP_BombaCopiaExplosiva_C" 0 _returnvalue "0, 0, 0" false self)))
            (Variables|Default|SetAtacar true)
            (Audio|PlaySoundatLocation "/Game/Marcos/Sons/pegarItem.pegarItem" "0, 0, 0" "0, 0, 0" 1.0 1.0 0.0 0 0 0)
            (Utilities|FlowControl|Delay 0.3)
            (Variables|Default|SetAtacar false)
            (Utilities|FlowControl|Delay 2.0)
            (Variables|Default|SetBombasGastas 0)
            (else
              (Variables|Default|SetBombasGastas (- (Variables|Default|GetBombasGastas) 1)))))))))

(fn ConstructionScript)