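; Explosive-copy bomb pawn of the BomberMago character, steered by its owner's movement input.
; On BeginPlay it copies the owner's strength value and binds to the move-right and move-forward dispatchers on the owner's BP_MagoPC controller.
; Each axis value, scaled by a speed multiplier, drives forced movement along fixed negative world Y and X axes.
; No explosion logic is defined in these graphs.
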(event Custom|MoveRight
  (params (AxisValue :type Float%20%28single-precision%29))
  (Pawn|Input|AddMovementInput "0.000000,-1.000000, 0" (* AxisValue (Variables|Default|GetMultiplicadoVelocidade)) true))

(event Custom|MoveForward
  (params (AxisValue :type Float%20%28single-precision%29))
  (Pawn|Input|AddMovementInput "-1.000000, 0, 0" (* AxisValue (Variables|Default|GetMultiplicadoVelocidade)) true))

(event EventBeginPlay
  (|CallParentFunction)
  (bind _asbp_bomber_mago (Utilities|Casting|CastToBP_BomberMago (Components|GetOwner)))
  (Variables|Default|SetForça (Variables|/Game/Marcos/Blueprints/BP_BomberMago.BP_BomberMago_C|GetForçah _asbp_bomber_mago))
  (bind _asbp_mago_pc (Utilities|Casting|CastToBP_MagoPC (Pawn|GetController _asbp_bomber_mago)))
  (bind _output_get (Variables|Default|SetOwnerPlayerController _asbp_mago_pc))
  (EventDispatchers|BindEventtoMoverRightEvent _output_get (delegate Custom|MoveRight))
  (EventDispatchers|BindEventtoMoverForwardEvent (Variables|Default|GetOwnerPlayerController) (delegate Custom|MoveForward)))

(fn ConstructionScript
  (|CallParentFunction))