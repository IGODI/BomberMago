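; GameMode_Mago is the game mode that sets up local multiplayer and switches between split-screen and shared-screen play.
; On BeginPlay it reads TelaCompartilhada from Bp_GameInstance to disable split-screen and show the shared-screen widget, then creates a local player.
; ReceberControlador stores the controller, and ReceberCamera stores the level camera.
; In shared-screen mode both point stored controllers' view at that camera, which CameraPrincipal returns.
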(event EventBeginPlay
  (Utilities|FlowControl|Sequence
    (:then_0
      (bind _asbp_game_instance (Utilities|Casting|CastToBp_GameInstance (Game|GetGameInstance)))
      (bind _output_get (Variables|Default|SetGameInstance _asbp_game_instance))
      (Class|GameplayStatics|SetForceDisableSplitscreen (Variables|/Game/Marcos/Blueprints/UI/Bp_GameInstance.Bp_GameInstance_C|GetTelaCompartilhada _output_get))
      (if (Variables|/Game/Marcos/Blueprints/UI/Bp_GameInstance.Bp_GameInstance_C|GetTelaCompartilhada _output_get)
        (bind _returnvalue (UserInterface|CreateWidget "/Game/Marcos/Blueprints/UI/HUDS/TelaCompartilhada.TelaCompartilhada_C"))
        (bind _output_get_2 (Variables|Default|SetInterfaceCompartilhada _returnvalue))
        (UserInterface|Viewport|AddtoViewport _output_get_2 0)))
    (:then_1
      (bind _returnvalue_2 (Class|GameplayStatics|CreatePlayer -1))
      (bind _asbp_mago_pc (Utilities|Casting|CastToBP_MagoPC _returnvalue_2))
      (CallFunction|ReceberControlador _asbp_mago_pc))))

(fn ConstructionScript)

(fn ReceberControlador
  (params (Novo%20Controlador :type BP%20Mago%20PC%20Object%20Reference))
  (bind _asbp_game_instance (Utilities|Casting|CastToBp_GameInstance (Game|GetGameInstance)))
  (Variables|Default|SetListaDeJogadores (Utilities|Array|MakeArray Novo%20Controlador))
  (Utilities|FlowControl|Sequence
    (:then_0
      (if (Variables|/Game/Marcos/Blueprints/UI/Bp_GameInstance.Bp_GameInstance_C|GetTelaCompartilhada _asbp_game_instance)
        (Variables|Default|GetCamera%20da%20Fase
          (:then
            (Game|Player|SetViewTargetwithBlend (Variables|Default|GetListaDeJogadores) (Variables|Default|GetCamera%20da%20Fase) 0.0 "VTBlend_Linear" 0.0 false))
          (:else))))))

(fn ReceberCamera
  (params (NovaCamera :type BP%20Camera%20Object%20Reference) (CameraDoPlayer :type %20Object%20Reference))
  (bind _asbp_game_instance (Utilities|Casting|CastToBp_GameInstance (Game|GetGameInstance)))
  (Variables|Default|SetCamera%20da%20Fase NovaCamera)
  (if (Variables|/Game/Marcos/Blueprints/UI/Bp_GameInstance.Bp_GameInstance_C|GetTelaCompartilhada _asbp_game_instance)
    (Game|Player|SetViewTargetwithBlend (Variables|Default|GetListaDeJogadores) (Variables|Default|GetCamera%20da%20Fase) 0.0 "VTBlend_Linear" 0.0 false)))

(fn CameraPrincipal
  (return (Variables|Default|GetCamera%20da%20Fase)))